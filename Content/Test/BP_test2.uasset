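; BP_test2 is a player-controlled test Blueprint with a pause-menu key and leftover directional obstacle-detection logic.
; P opens BP_pauseMenu, switches to UI-only input and pauses the game, while BeginPlay adds the Enhanced Input mapping context.
; WASD only stores a direction offset, and the input action event is empty.
; The box trace using that offset, which flashes the cube red then green through dynamic materials, is disconnected and never runs.
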(event Input|EnhancedActionEvents|EnhancedInputActionAI_InputDirection
  (params (ActionValue :type Vector%202D%20Structure) (ElapsedSeconds :type Float%20%28double-precision%29) (TriggeredSeconds :type Float%20%28double-precision%29) (InputAction :type Input%20Action%20Object%20Reference :default "/Game/AI_InputDirection.AI_InputDirection")))

(event EventBeginPlay
  (bind _asplayer_controller (Utilities|Casting|CastToPlayerController (Pawn|GetController)))
  (Input|AddMappingContext (PlayerController|LocalPlayerSubsystems|GetEnhancedInputLocalPlayerSubsystem _asplayer_controller) "/Game/IMC.IMC" 0 "(bIgnoreAllPressedKeysUntilRelease=True,bForceImmediately=False,bNotifyUserSettings=False)"))

(event Input|KeyboardEvents|P
  (params (Key :type Key%20Structure :default "None"))
  (bind _returnvalue (Game|GetPlayerController 0))
  ;[0.15 0.15 0.15 0.5] Menu
  (:Pressed
    (bind _returnvalue_2 (UserInterface|CreateWidget "/Game/Lvs/BP_pauseMenu.BP_pauseMenu_C"))
    (UserInterface|Viewport|AddtoViewport _returnvalue_2 0)
    (Variables|/Script/Engine.PlayerController|SetbShowMouseCursor _returnvalue true)
    (Input|SetInputModeUIOnly _returnvalue 0 "DoNotLock" false)
    (Game|SetGamePaused true)))

(event Input|KeyboardEvents|W
  (params (Key :type Key%20Structure :default "None"))
  (:Pressed
    (Variables|Default|SetLenght "100.000000,0.000000,0.000000")))

(event Input|KeyboardEvents|S
  (params (Key :type Key%20Structure :default "None"))
  (:Pressed
    (Variables|Default|SetLenght "-100.000000,0.000000,0.000000")))

(event Input|KeyboardEvents|A
  (params (Key :type Key%20Structure :default "None"))
  (:Pressed
    (Variables|Default|SetLenght "0.000000,-100.000000,-0.000000")))

(event Input|KeyboardEvents|D
  (params (Key :type Key%20Structure :default "None"))
  (:Pressed
    (Variables|Default|SetLenght "0.000000,100.000000,0.000000")))

(fn ConstructionScript)