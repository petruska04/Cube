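; Test cube actor that rolls step by step with WASD and opens a pause menu on P.
; Each key box-traces ahead from the actor location, flashing the cube red then green via dynamic materials if blocked.
; Otherwise input locks while the Sphere shifts as a pivot, the Cube attaches and a per-direction Timeline rotates it.
; On finish the Cube detaches and the pivot resets rotation; only D also moves the actor.
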(event EventBeginPlay
  (Input|EnableInput (Game|GetPlayerController 0)))

(event Input|KeyboardEvents|P
  (params (Key :type Key%20Structure :default "None"))
  (bind _returnvalue (Game|GetPlayerController 0))
  ;[0.15 0.15 0.15 0.5] Menu
  (:Pressed
    (bind _returnvalue_2 (UserInterface|CreateWidget "/Game/Lvs/BP_pauseMenu.BP_pauseMenu_C"))
    (UserInterface|Viewport|AddtoViewport _returnvalue_2 0)
    (Variables|/Script/Engine.PlayerController|SetbShowMouseCursor _returnvalue true)
    (Input|SetInputModeUIOnly _returnvalue 0 "DoNotLock" false)
    (Game|SetGamePaused true)))

(event Input|KeyboardEvents|W
  (params (Key :type Key%20Structure :default "None"))
  (bind _returnvalue (Transformation|GetActorLocation))
  (bind _returnvalue_2 (+ _returnvalue "0.000000,0.000000,50.000000"))
  (:Pressed
    (Variables|Default|SetLenght "100.000000,0.000000,0.000000")
    (Utilities|FlowControl|Delay 0.01)
    (bind _returnvalue_3 (Collision|BoxTraceByChannel _returnvalue_2 (+ _returnvalue_2 (Variables|Default|GetLenght)) "40.000000,40.000000,40.000000" "0, 0, 0" "TraceTypeQuery1" false 0 "ForDuration"))
    (if _returnvalue_3
      (CallFunction|ChangColorRed)
      (Utilities|FlowControl|Delay 0.2)
      (CallFunction|ChangColorGreen)
      (else
        (Input|DisableInput (Game|GetPlayerController 0))
        (Transformation|AddRelativeLocation (Variables|Default|GetSphere) "0.000000,-50.000000,0.000000" false false)
        (Transformation|AttachComponentToComponent (Variables|Default|GetCube) (Variables|Default|GetSphere) "None" "KeepWorld" "KeepWorld" "KeepWorld" true)
        (bind _newtrack_0 (Timeline|Timeline_1 PlayFromStart)
          (:Update
            (Transformation|SetRelativeRotation (Variables|Default|GetSphere) (Math|Rotator|MakeRotator _newtrack_0 0.0 0.0) false false))
          (:Finished
            (Transformation|DetachFromComponent (Variables|Default|GetCube) "KeepWorld" "KeepWorld" "KeepWorld" true)
            (Transformation|AddRelativeLocation (Variables|Default|GetSphere) "0.000000,-50.000000,0.000000" false false)
            (Transformation|SetRelativeRotation (Variables|Default|GetSphere) "0, 0, 0" false false)
            (Input|EnableInput (Game|GetPlayerController 0))))))))

(event Input|KeyboardEvents|A
  (params (Key :type Key%20Structure :default "None"))
  (bind _returnvalue (Transformation|GetActorLocation))
  (bind _returnvalue_2 (+ _returnvalue "0.000000,0.000000,50.000000"))
  (:Pressed
    (Development|PrintString (Utilities|String|ToString(Vector) (Transformation|GetActorLocation)))
    (Variables|Default|SetLenght "0.000000,-100.000000,0.000000")
    (Utilities|FlowControl|Delay 0.01)
    (bind _returnvalue_3 (Collision|BoxTraceByChannel _returnvalue_2 (+ _returnvalue_2 (Variables|Default|GetLenght)) "40.000000,40.000000,40.000000" "0, 0, 0" "TraceTypeQuery1" false 0 "ForDuration"))
    (if _returnvalue_3
      (CallFunction|ChangColorRed)
      (Utilities|FlowControl|Delay 0.2)
      (CallFunction|ChangColorGreen)
      (else
        (Input|DisableInput (Game|GetPlayerController 0))
        (Transformation|AddRelativeLocation (Variables|Default|GetSphere) "-50.000000,0.000000,0.000000" false false)
        (Transformation|AttachComponentToComponent (Variables|Default|GetCube) (Variables|Default|GetSphere) "None" "KeepWorld" "KeepWorld" "KeepWorld" true)
        (bind _newtrack_0 (Timeline|Timeline_0 PlayFromStart)
          (:Update
            (Transformation|SetRelativeRotation (Variables|Default|GetSphere) (Math|Rotator|MakeRotator 0.0 _newtrack_0 0.0) false false))
          (:Finished
            (Transformation|DetachFromComponent (Variables|Default|GetCube) "KeepWorld" "KeepWorld" "KeepWorld" true)
            (Transformation|AddRelativeLocation (Variables|Default|GetSphere) "-50.000000,0.000000,0.000000" false false)
            (Transformation|SetRelativeRotation (Variables|Default|GetSphere) "0, 0, 0" false false)
            (Input|EnableInput (Game|GetPlayerController 0))))))))

(event Input|KeyboardEvents|S
  (params (Key :type Key%20Structure :default "None"))
  (bind _returnvalue (Transformation|GetActorLocation))
  (bind _returnvalue_2 (+ _returnvalue "0.000000,0.000000,50.000000"))
  (:Pressed
    (Variables|Default|SetLenght "-100.000000,0.000000,0.000000")
    (Utilities|FlowControl|Delay 0.01)
    (bind _returnvalue_3 (Collision|BoxTraceByChannel _returnvalue_2 (+ _returnvalue_2 (Variables|Default|GetLenght)) "40.000000,40.000000,40.000000" "0, 0, 0" "TraceTypeQuery1" false 0 "None"))
    (if _returnvalue_3
      (CallFunction|ChangColorRed)
      (Utilities|FlowControl|Delay 0.2)
      (CallFunction|ChangColorGreen)
      (else
        (Input|DisableInput (Game|GetPlayerController 0))
        (Transformation|AddRelativeLocation (Variables|Default|GetSphere) "0.000000,50.000000,0.000000" false false)
        (Transformation|AttachComponentToComponent (Variables|Default|GetCube) (Variables|Default|GetSphere) "None" "KeepWorld" "KeepWorld" "KeepWorld" true)
        (bind _newtrack_0 (Timeline|Timeline_2 PlayFromStart)
          (:Update
            (Transformation|SetRelativeRotation (Variables|Default|GetSphere) (Math|Rotator|MakeRotator _newtrack_0 0.0 0.0) false false))
          (:Finished
            (Transformation|DetachFromComponent (Variables|Default|GetCube) "KeepWorld" "KeepWorld" "KeepWorld" true)
            (Transformation|AddRelativeLocation (Variables|Default|GetSphere) "0.000000,50.000000,0.000000" false false)
            (Transformation|SetRelativeRotation (Variables|Default|GetSphere) "0, 0, 0" false false)
            (Input|EnableInput (Game|GetPlayerController 0))))))))

(event Input|KeyboardEvents|D
  (params (Key :type Key%20Structure :default "None"))
  (bind _returnvalue (Transformation|GetActorLocation))
  (bind _returnvalue_2 (+ _returnvalue "0.000000,0.000000,50.000000"))
  (:Pressed
    (Variables|Default|SetLenght "0.000000,100.000000,0.000000")
    (Utilities|FlowControl|Delay 0.01)
    (bind _returnvalue_3 (Collision|BoxTraceByChannel _returnvalue_2 (+ _returnvalue_2 (Variables|Default|GetLenght)) "40.000000,40.000000,40.000000" "0, 0, 0" "TraceTypeQuery1" false 0 "ForDuration"))
    (if _returnvalue_3
      (CallFunction|ChangColorRed)
      (Utilities|FlowControl|Delay 0.2)
      (CallFunction|ChangColorGreen)
      (else
        (Input|DisableInput (Game|GetPlayerController 0))
        (Transformation|AddRelativeLocation (Variables|Default|GetSphere) "50.000000,0.000000,0.000000" false false)
        (Transformation|AttachComponentToComponent (Variables|Default|GetCube) (Variables|Default|GetSphere) "None" "KeepWorld" "KeepWorld" "KeepWorld" true)
        (bind _newtrack_0 (Timeline|Timeline PlayFromStart)
          (:Update
            (Transformation|SetRelativeRotation (Variables|Default|GetSphere) (Math|Rotator|MakeRotator 0.0 _newtrack_0 0.0) false false))
          (:Finished
            (Transformation|DetachFromComponent (Variables|Default|GetCube) "KeepWorld" "KeepWorld" "KeepWorld" true)
            (Transformation|AddRelativeLocation (Variables|Default|GetSphere) "50.000000,0.000000,0.000000" false false)
            (Transformation|SetRelativeRotation (Variables|Default|GetSphere) "0, 0, 0" false false)
            (Transformation|SetActorLocation (+ (Transformation|GetActorLocation) "50.000000,0.000000,0.000000") false true)
            (Input|EnableInput (Game|GetPlayerController 0))))))))

(fn ConstructionScript)

(fn MoveW)

(fn ChangColorRed
  (bind _returnvalue (Rendering|Material|CreateDynamicMaterialInstance "/Game/Fab/Box/box/Materials/initialShadingGroup.initialShadingGroup" "None" "None" :!class /Script/Engine.KismetMaterialLibrary))
  (Rendering|Material|SetMaterial (Variables|Default|GetCube) 0 _returnvalue)
  (bind _output_get (Variables|Default|SetNewVar _returnvalue))
  (Rendering|Material|SetVectorParameterValue _output_get "EmissiveFactor" (Math|Color|MakeColor 1.0 0.0 0.0) :!class /Script/Engine.MaterialInstanceDynamic))

(fn ChangColorGreen
  (bind _returnvalue (Rendering|Material|CreateDynamicMaterialInstance "/Game/Fab/Box/box/Materials/initialShadingGroup.initialShadingGroup" "None" "None" :!class /Script/Engine.KismetMaterialLibrary))
  (Rendering|Material|SetMaterial (Variables|Default|GetCube) 0 _returnvalue)
  (bind _output_get (Variables|Default|SetNewVar_0 _returnvalue))
  (Rendering|Material|SetVectorParameterValue _output_get "EmissiveFactor" (Math|Color|MakeColor 0.0 1.0 0.0 0.0) :!class /Script/Engine.MaterialInstanceDynamic))