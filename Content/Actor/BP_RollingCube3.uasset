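; Player-controlled cube pawn that rolls a quarter turn about its bottom edge per Enhanced Input move, with P opening a pause menu.
; WASD keys set a height-dependent trace offset, which the move input line-traces after a brief delay.
; A hit blocks the move and flashes the cube red, then green, via dynamic materials.
; Otherwise it computes pivot and axis, and Tick rotates it with sweep, snapping rotation at 90 degrees.
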(event Input|EnhancedActionEvents|EnhancedInputActionAI_InputDirection
  (params (ActionValue :type Vector%202D%20Structure) (ElapsedSeconds :type Float%20%28double-precision%29) (TriggeredSeconds :type Float%20%28double-precision%29) (InputAction :type Input%20Action%20Object%20Reference :default "/Game/AI_InputDirection.AI_InputDirection"))
  (bind _returnvalue (Transformation|GetActorLocation))
  (bind (_x _y) (Math|Vector2D|BreakVector2D ActionValue))
  (bind _cube (Variables|Default|GetCube))
  (bind (_origin _boxextent) (Collision|GetComponentBounds _cube))
  (Utilities|FlowControl|Delay 0.01)
  (bind _returnvalue_2 (Collision|LineTraceByChannel _returnvalue (+ _returnvalue (Variables|Default|GetX)) "TraceTypeQuery1" false 0 "None"))
  (if _returnvalue_2
    (bind _returnvalue_3 (Rendering|Material|CreateDynamicMaterialInstance "/Game/Fab/Box/box/Materials/initialShadingGroup.initialShadingGroup" "None" "None" :!class /Script/Engine.KismetMaterialLibrary))
    (Rendering|Material|SetMaterial (Variables|Default|GetCube) 0 _returnvalue_3)
    (bind _output_get (Variables|Default|SetNewVar _returnvalue_3))
    (Rendering|Material|SetVectorParameterValue _output_get "EmissiveFactor" (Math|Color|MakeColor 1.0 0.0 0.0) :!class /Script/Engine.MaterialInstanceDynamic)
    (Utilities|FlowControl|Delay 0.2)
    (bind _returnvalue_4 (Rendering|Material|CreateDynamicMaterialInstance "/Game/Fab/Box/box/Materials/initialShadingGroup.initialShadingGroup" "None" "None" :!class /Script/Engine.KismetMaterialLibrary))
    (Rendering|Material|SetMaterial (Variables|Default|GetCube) 0 _returnvalue_4)
    (bind _output_get_2 (Variables|Default|SetNewVar_0 _returnvalue_4))
    (Rendering|Material|SetVectorParameterValue _output_get_2 "EmissiveFactor" (Math|Color|MakeColor 0.0 1.0 0.0 0.0) :!class /Script/Engine.MaterialInstanceDynamic)
    (elif (not (Variables|Default|GetRolling))
      (bind _output_get_3 (Variables|Default|SetInputDirection (Math|Vector|MakeVector _x _y 0.0)))
      (Variables|Default|SetPivotPoint (Math|Vector|MakeVector (.x (+ (* _output_get_3 _boxextent) _origin)) (.y (+ (* _output_get_3 _boxextent) _origin)) (- (.z (+ (* _output_get_3 _boxextent) _origin)) (.Z (Math|Vector|BreakVector _boxextent)))))
      (Variables|Default|SetAxisRotation (Math|Vector|RotateVectorAroundAxis (Variables|Default|GetInputDirection) 9e+01 "0.000000,0.000000,1.000000"))
      (Variables|Default|SetTargetRotation (Math|Rotator|CombineRotators (Transformation|GetActorRotation) (Math|Rotator|MakeRotator (* (.y (Variables|Default|GetInputDirection)) 9e+01) (* (* (.x (Variables|Default|GetInputDirection)) -1.0) 9e+01) 0.0)))
      (Variables|Default|SetRolling true))))

(event EventBeginPlay
  (bind _asplayer_controller (Utilities|Casting|CastToPlayerController (Pawn|GetController)))
  (Input|AddMappingContext (PlayerController|LocalPlayerSubsystems|GetEnhancedInputLocalPlayerSubsystem _asplayer_controller) "/Game/IMC.IMC" 0 "(bIgnoreAllPressedKeysUntilRelease=True,bForceImmediately=False,bNotifyUserSettings=False)"))

(event EventTick
  (params (DeltaSeconds :type Float%20%28single-precision%29))
  (if (Variables|Default|GetRolling)
    (if (>= (Variables|Default|GetCurrentAngel) 86.0)
      (Variables|Default|SetDeltaAngel (- 9e+01 (Variables|Default|GetCurrentAngel)))
      (else
        (Variables|Default|SetDeltaAngel (* (Variables|Default|GetRotationSpeed) DeltaSeconds))))
    (if (>= (Variables|Default|GetCurrentAngel) 9e+01)
      (Variables|Default|SetRolling false)
      (Variables|Default|SetCurrentAngel 0.0)
      (Transformation|SetActorRotation (Variables|Default|GetTargetRotation))
      (else
        (Transformation|SetActorLocationAndRotation (+ (Math|Vector|RotateVector (- (Transformation|GetActorLocation) (Variables|Default|GetPivotPoint)) (Math|Vector|RotatorfromAxisandAngle (Variables|Default|GetAxisRotation) (Variables|Default|GetDeltaAngel))) (Variables|Default|GetPivotPoint)) (Math|Rotator|CombineRotators (Transformation|GetActorRotation) (Math|Vector|RotatorfromAxisandAngle (Variables|Default|GetAxisRotation) (Variables|Default|GetDeltaAngel))) true)
        (Variables|Default|SetCurrentAngel (+ (Variables|Default|GetCurrentAngel) (Variables|Default|GetDeltaAngel)))))))

(event Input|KeyboardEvents|P
  (params (Key :type Key%20Structure :default "None"))
  (bind _returnvalue (Game|GetPlayerController 0))
  (:Pressed
    (bind _returnvalue_2 (UserInterface|CreateWidget "/Game/Lvs/BP_pauseMenu.BP_pauseMenu_C"))
    (UserInterface|Viewport|AddtoViewport _returnvalue_2 0)
    (Variables|/Script/Engine.PlayerController|SetbShowMouseCursor _returnvalue true)
    (Input|SetInputModeUIOnly _returnvalue 0 "DoNotLock" false)
    (Game|SetGamePaused true)))

(event Input|KeyboardEvents|W
  (params (Key :type Key%20Structure :default "None"))
  (:Pressed
    (if (<= (.z (Transformation|GetActorLocation)) 3e+02)
      (Variables|Default|SetX "150.000000,0.000000,-20.000000")
      (else
        (Variables|Default|SetX "250.000000,0.000000,-20.000000")))))

(event Input|KeyboardEvents|S
  (params (Key :type Key%20Structure :default "None"))
  (:Pressed
    (if (<= (.z (Transformation|GetActorLocation)) 3e+02)
      (Variables|Default|SetX "-150.000000,0.000000,-20.000000")
      (else
        (Variables|Default|SetX "-250.000000,0.000000,-20.000000")))))

(event Input|KeyboardEvents|A
  (params (Key :type Key%20Structure :default "None"))
  (:Pressed
    (if (<= (.z (Transformation|GetActorLocation)) 3e+02)
      (Variables|Default|SetX "10.000000,-150.000000,-20.000000")
      (else
        (Variables|Default|SetX "10.000000,-250.000000,-20.000000")))))

(event Input|KeyboardEvents|D
  (params (Key :type Key%20Structure :default "None"))
  (:Pressed
    (if (<= (.z (Transformation|GetActorLocation)) 3e+02)
      (Variables|Default|SetX "10.000000,150.000000,-20.000000")
      (else
        (Variables|Default|SetX "10.000000,250.000000,-20.000000")))))

(fn ConstructionScript)